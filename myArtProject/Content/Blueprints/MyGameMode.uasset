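; MyGameMode is a game mode that drives enemy spawning and movement.
; On BeginPlay it finds the first EnemySpawner and sets a looping timer that calls its SpawnEnemy function at the EnemiesPerSecond rate.
; Every Tick it gathers all Enemy2 actors and moves each down the Z axis by a fixed, frame-rate-dependent step, resetting rotation and scale.
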(event EventBeginPlay
  ;[1 1 1] Spawns an Enemy based on time
  (bind _outactors (Actor|GetAllActorsOfClass "/Game/Blueprints/EnemySpawner.EnemySpawner_C"))
  (bind _output_get (Variables|Default|SetEnemySpawner (Utilities|Array|Get(acopy) _outactors)))
  (Utilities|Time|SetTimerbyFunctionName _output_get "SpawnEnemy" (/ 1.0 (Variables|Default|GetEnemiesPerSecond)) true))

(event EventTick
  (params (DeltaSeconds :type Float%20%28single-precision%29))
  ;[1 1 1] Enemy Movement
  (bind _outactors (Actor|GetAllActorsOfClass "/Game/Blueprints/Enemy2.Enemy2_C"))
  (for _array_element _outactors
    (Transformation|SetActorTransform _array_element (Math|Transform|MakeTransform (- (Transformation|GetActorLocation _array_element) "0, 0,1.000000")))))

(fn ConstructionScript)