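; Enemy2 is a clickable Paper2D sprite enemy that applies a color-change material on BeginPlay.
; A click or touch destroys it, adding to the game mode's score if it is flagged IsRegular.
; Overlapping a HitBox also destroys it; regular ones reduce TotalHealth and quit the game once that drops below zero.
; Tick casts its widget to EnemyUI without using the result.
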(event OnClicked(PaperSprite)
  (params (TouchedComponent :type Primitive%20Component%20Object%20Reference) (ButtonPressed :type Key%20Structure))
  ;[1 1 1] Destroys Enemy when clicked
  (Actor|DestroyActor)
  (if (Variables|Default|GetIsRegular)
    ;[1 1 1] Add 1 to score if the correct language was destroyed
    (bind _asmy_game_mode (Utilities|Casting|CastToMyGameMode (Game|GetGameMode)))
    (Variables|/Game/Blueprints/MyGameMode.MyGameMode_C|SetCurrentScore _asmy_game_mode (+ (Variables|/Game/Blueprints/MyGameMode.MyGameMode_C|GetCurrentScore _asmy_game_mode) 1))))

(event EventBeginPlay
  (Rendering|Material|SetMaterialbyName (Variables|Default|GetPaperSprite) "None" "/Game/Materials/ColorChange2.ColorChange2"))

(event Collision|EventActorBeginOverlap
  (params (OtherActor :type Actor%20Object%20Reference))
  ;[1 1 1] When enemy hits bottom it: Destroys itself, Decraments Total Health (if bad language)
  (Utilities|Casting|CastToHitBox OtherActor)
  (Actor|DestroyActor)
  (if (Variables|Default|GetIsRegular)
    (bind _asmy_game_mode (Utilities|Casting|CastToMyGameMode (Game|GetGameMode)))
    (Variables|/Game/Blueprints/MyGameMode.MyGameMode_C|SetTotalHealth _asmy_game_mode (- (Variables|/Game/Blueprints/MyGameMode.MyGameMode_C|GetTotalHealth _asmy_game_mode) 1))
    ;[1 1 1] Quit Game if health is less than 0
    (if (< (Variables|/Game/Blueprints/MyGameMode.MyGameMode_C|GetTotalHealth _asmy_game_mode) 0)
      (Game|QuitGame 0 "Quit"))))

(event EventTick
  (params (DeltaSeconds :type Float%20%28single-precision%29))
  (bind _asenemy_ui (Utilities|Casting|CastToEnemyUI (UserInterface|GetUserWidgetObject (Variables|Default|GetEnemyWidget)))))

(event EventActorOnInputTouchBegin
  (params (FingerIndex :type ETouchIndex%20Enum :default "Touch1"))
  ;[1 1 1] Destroys Enemy when clicked
  (Actor|DestroyActor)
  (if (Variables|Default|GetIsRegular)
    ;[1 1 1] Add 1 to score if the correct language was destroyed
    (bind _asmy_game_mode (Utilities|Casting|CastToMyGameMode (Game|GetGameMode)))
    (Variables|/Game/Blueprints/MyGameMode.MyGameMode_C|SetCurrentScore _asmy_game_mode (+ (Variables|/Game/Blueprints/MyGameMode.MyGameMode_C|GetCurrentScore _asmy_game_mode) 1))))

(fn ConstructionScript)